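; Elevator actor that the player toggles with E while inside its trigger box, which enables and disables input on overlap.
; A FlipFlop plays or reverses a timeline that drives the elevator's relative location.
; Releasing E fades in elevator music, or re-triggers the FlipFlop if music is already playing.
; The music stops when the timeline finishes.
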(event OnComponentBeginOverlap(Box)
  (params (OverlappedComponent :type Primitive%20Component%20Object%20Reference) (OtherActor :type Actor%20Object%20Reference) (OtherComp :type Primitive%20Component%20Object%20Reference) (OtherBodyIndex :type Integer) (bFromSweep :type Boolean) (SweepResult :type Hit%20Result%20Structure%20%28by%20ref%29))
  (Input|EnableInput (Game|GetPlayerController 0)))

(event OnComponentEndOverlap(Box)
  (params (OverlappedComponent :type Primitive%20Component%20Object%20Reference) (OtherActor :type Actor%20Object%20Reference) (OtherComp :type Primitive%20Component%20Object%20Reference) (OtherBodyIndex :type Integer))
  (Input|DisableInput (Game|GetPlayerController 0)))

(event EventBeginPlay)

(event Collision|EventActorBeginOverlap
  (params (OtherActor :type Actor%20Object%20Reference)))

(event EventTick
  (params (DeltaSeconds :type Float%20%28single-precision%29)))

(event Input|KeyboardEvents|E
  (params (Key :type Key%20Structure :default "None"))
  (bind _elevator_music__kevin_macleod____background_music__hd__cue (Variables|Default|GetElevator_Music__Kevin_MacLeod__-_Background_Music__HD__Cue))
  (:Pressed
    (Utilities|FlowControl|FlipFlop :!label _label
      (:A
        (bind _newtrack_0 (Timeline|elevatorTimeLine Play)
          (:Update
            (Transformation|SetRelativeLocation (Variables|Default|Getelvator) _newtrack_0 false false))
          (:Finished
            (Audio|Components|Audio|Stop (Variables|Default|GetElevator_Music__Kevin_MacLeod__-_Background_Music__HD__Cue)))))
      (:B
        (Timeline|elevatorTimeLine Reverse))))
  (:Released
    (if (Audio|Components|Audio|IsPlaying _elevator_music__kevin_macleod____background_music__hd__cue)
      (goto _label)
      (else
        (Audio|Components|Audio|FadeIn _elevator_music__kevin_macleod____background_music__hd__cue 0.0 1.0 0.0 "Linear" :!class /Script/Engine.AudioComponent)))))

(fn ConstructionScript)